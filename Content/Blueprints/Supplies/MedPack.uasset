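; MedPack is a health pickup that heals a Base_Character when it touches the pack's capsule.
; On overlap, a character below full health gains the HealthGiven amount, read through GiveHealth and clamped to the health cap, and the pack destroys itself.
; Characters already at full health leave the pack in place.
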(event `self.Capsule.OnComponentBeginOverlap`
  (params (OverlappedComponent :type "PrimitiveComponent Object Reference") (OtherActor :type "Actor Object Reference") (OtherComp :type "PrimitiveComponent Object Reference") (OtherBodyIndex :type Integer) (bFromSweep :type Boolean) (SweepResult :type "HitResult Structure (by ref)"))
  (bind _asbase_character (cast `/Game/Blueprints/Characters/Base_Character` OtherActor))
  (bind _health (`/Game/Blueprints/Characters/Base_Character.Health` _asbase_character))
  (if (< _health 100.0)
    (bind _heal (`self.GiveHealth`))
    (set `/Game/Blueprints/Characters/Base_Character.Health` (`KismetMathLibrary.FClamp` (+ _heal _health) 0.0 100.0) _asbase_character)
    (`self.K2_DestroyActor`)))

(fn `GiveHealth`
  (returns (Heal :type "Float (double-precision)"))
  (return (`self.HealthGiven`)))

(fn `UserConstructionScript`
  (`parent.UserConstructionScript`))
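; AmmoBox is a supply pickup that refills a character's gun when walked into.
; On Box overlap it casts the actor to Base_Character and reads the Clip component on that character's GunRef.
; If the clip holds less than its maximum, it adds a fixed amount of ammo, clamped to that maximum, and destroys itself.
; A full clip leaves the box in place.
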(event `self.Box.OnComponentBeginOverlap`
  (params (OverlappedComponent :type "PrimitiveComponent Object Reference") (OtherActor :type "Actor Object Reference") (OtherComp :type "PrimitiveComponent Object Reference") (OtherBodyIndex :type Integer) (bFromSweep :type Boolean) (SweepResult :type "HitResult Structure (by ref)"))
  (bind _asbase_character (cast `/Game/Blueprints/Characters/Base_Character` OtherActor))
  (bind _returnvalue (`self.GetComponentByClass` (`/Game/Blueprints/Characters/Base_Character.GunRef` _asbase_character) "/Game/Blueprints/Supplies/Clip.Clip_C"))
  (bind _maxammotohold (`/Game/Blueprints/Supplies/Clip.MaxAmmoToHold` _returnvalue))
  (if (< (`/Game/Blueprints/Supplies/Clip.CurrentAmmoHolding` _returnvalue) _maxammotohold)
    (`/Game/Blueprints/Supplies/Clip.AddAmmo` _returnvalue (`KismetMathLibrary.Clamp` 15 0 _maxammotohold))
    (`self.K2_DestroyActor`)))

(fn `UserConstructionScript`
  (`parent.UserConstructionScript`))
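; Ammo supply shelf that refills the held non-melee gun when a character overlaps its box and the clip isn't full.
; Each overlap hides the first available of six child-actor boxes, decrements the shelf's stock and adds a fixed amount to the weapon's clip.
; Tick re-shows taken boxes after a short delay while enough stock remains for that slot.
; Stock starts at MaxAmmo, and Taken flags are never cleared.
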(event `self.Box.OnComponentBeginOverlap`
  (params (OverlappedComponent :type "PrimitiveComponent Object Reference") (OtherActor :type "Actor Object Reference") (OtherComp :type "PrimitiveComponent Object Reference") (OtherBodyIndex :type Integer) (bFromSweep :type Boolean) (SweepResult :type "HitResult Structure (by ref)"))
  (bind _childactor (`self.ChildActor`))
  (bind _childactor1 (`self.ChildActor1`))
  (bind _childactor2 (`self.ChildActor2`))
  (bind _childactor3 (`self.ChildActor3`))
  (bind _childactor4 (`self.ChildActor4`))
  (bind _childactor5 (`self.ChildActor5`))
  ;[1 1 1] Remove boxes after taking
  (bind _asbase_character (cast `/Game/Blueprints/Characters/Base_Character` OtherActor))
  (bind _gunref (`/Game/Blueprints/Characters/Base_Character.GunRef` _asbase_character))
  (`/Engine/EditorBlueprintResources/StandardMacros.IsValid` _gunref
    (:`Is Valid`
      (bind _asmaster_weapon (cast `/Game/Blueprints/Supplies/WeaponBP/Master_Weapon` _gunref))
      (if (not (`/Game/Blueprints/Supplies/WeaponBP/Master_Weapon.IsMelee?` _asmaster_weapon))
        (bind _clip (`/Game/Blueprints/Supplies/WeaponBP/Master_Weapon.Clip` _asmaster_weapon))
        (if (< (`/Game/Blueprints/Supplies/Clip.CurrentAmmoHolding` _clip) (`/Game/Blueprints/Supplies/Clip.MaxAmmoToHold` _clip))
          (if (`SceneComponent.IsVisible` _childactor)
            (`SceneComponent.SetVisibility` (`self.ChildActor`) false false)
            (set `self.CurrentAmmo` (- (`self.CurrentAmmo`) 1))
            (set `self.Taken1` true)
            (`/Game/Blueprints/Supplies/Clip.AddAmmo` _clip 15)
            (elif (and (not (`SceneComponent.IsVisible` _childactor)) (`SceneComponent.IsVisible` _childactor1))
              (`SceneComponent.SetVisibility` (`self.ChildActor1`) false false)
              (set `self.CurrentAmmo` (- (`self.CurrentAmmo`) 1))
              (set `self.Taken2` true)
              (`/Game/Blueprints/Supplies/Clip.AddAmmo` _clip 15)
              (elif (and (not (`SceneComponent.IsVisible` _childactor1)) (`SceneComponent.IsVisible` _childactor2))
                (`SceneComponent.SetVisibility` _childactor2 false false)
                (set `self.CurrentAmmo` (- (`self.CurrentAmmo`) 1))
                (set `self.Taken3` true)
                (`/Game/Blueprints/Supplies/Clip.AddAmmo` _clip 15)
                (elif (and (not (`SceneComponent.IsVisible` _childactor2)) (`SceneComponent.IsVisible` _childactor3))
                  (`SceneComponent.SetVisibility` (`self.ChildActor3`) false false)
                  (set `self.CurrentAmmo` (- (`self.CurrentAmmo`) 1))
                  (set `self.Taken4` true)
                  (`/Game/Blueprints/Supplies/Clip.AddAmmo` _clip 15)
                  (elif (and (not (`SceneComponent.IsVisible` _childactor3)) (`SceneComponent.IsVisible` _childactor4))
                    (`SceneComponent.SetVisibility` _childactor4 false false)
                    (set `self.CurrentAmmo` (- (`self.CurrentAmmo`) 1))
                    (set `self.Taken5` true)
                    (`/Game/Blueprints/Supplies/Clip.AddAmmo` _clip 15)
                    (elif (and (not (`SceneComponent.IsVisible` _childactor4)) (`SceneComponent.IsVisible` _childactor5))
                      (`SceneComponent.SetVisibility` _childactor5 false false)
                      (set `self.CurrentAmmo` (- (`self.CurrentAmmo`) 1))
                      (set `self.Taken6` true)
                      (`/Game/Blueprints/Supplies/Clip.AddAmmo` _clip 15))))))))))))

(event `self.ReceiveBeginPlay`
  (set `self.CurrentAmmo` (`self.MaxAmmo`)))

(event `self.ReceiveTick`
  (params (DeltaSeconds :type "Float (single-precision)"))
  (if (not (== (`self.CurrentAmmo`) 0))
    (`|ExecutionSequence`
      (:`then_0`
        (if (`self.Taken1`)
          (if (> (`self.CurrentAmmo`) 0)
            (`KismetSystemLibrary.Delay` 2.0)
            (`SceneComponent.SetVisibility` (`self.ChildActor`) true false))))
      (:`then_1`
        (if (`self.Taken2`)
          (if (> (`self.CurrentAmmo`) 1)
            (`KismetSystemLibrary.Delay` 2.0)
            (`SceneComponent.SetVisibility` (`self.ChildActor1`) true false))))
      (:`then_2`
        (if (`self.Taken3`)
          (if (> (`self.CurrentAmmo`) 2)
            (`KismetSystemLibrary.Delay` 2.0)
            (`SceneComponent.SetVisibility` (`self.ChildActor2`) true false))))
      (:`then_3`
        (if (`self.Taken4`)
          (if (> (`self.CurrentAmmo`) 3)
            (`KismetSystemLibrary.Delay` 2.0)
            (`SceneComponent.SetVisibility` (`self.ChildActor3`) true false))))
      (:`then_4`
        (if (`self.Taken5`)
          (if (> (`self.CurrentAmmo`) 4)
            (`KismetSystemLibrary.Delay` 2.0)
            (`SceneComponent.SetVisibility` (`self.ChildActor4`) true false))))
      (:`then_5`
        (if (`self.Taken6`)
          (if (> (`self.CurrentAmmo`) 5)
            (`KismetSystemLibrary.Delay` 2.0)
            (`SceneComponent.SetVisibility` (`self.ChildActor5`) true false)))))))

(fn `UserConstructionScript`)
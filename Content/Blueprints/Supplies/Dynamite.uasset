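; Dynamite supply actor that arms, counts down and explodes, damaging overlapping actors before destroying itself.
; A Base_Character with IndexNumber 4 shooting inside its Box arms it and briefly shows a warning widget to player 0.
; Delays on Tick act as one-second timers, decrementing Count while a FlipFlop blinks the PointLight.
; At zero, serverdamage spawns the explosion and applies damage; a separate ShowAgain event restores visibility.
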(event `serverdamage`
  (bind _output_get (set `self.Place` (`SceneComponent.K2_GetComponentLocation` (`self.Dyna`))))
  (`KismetSystemLibrary.Delay` 0.2)
  (`GameplayStatics.SpawnEmitterAtLocation` "/Game/Particles/P_Explosion.P_Explosion" _output_get (struct) (2.0 2.0 2.0))
  (for _array_element (`self.GetOverlappingActors` self "/Script/Engine.Actor")
    (`GameplayStatics.ApplyDamage` _array_element 500.0 null null "/Script/Engine.DamageType")
    (`KismetSystemLibrary.Delay` 0.2)
    (`self.K2_DestroyActor`)))

(event `self.ReceiveTick`
  (params (DeltaSeconds :type "Float (single-precision)"))
  (`parent.ReceiveTick` DeltaSeconds)
  (`|ExecutionSequence`
    (:`then_0`
      (`KismetSystemLibrary.Delay` 1.0)
      (if (`self.Blink?`)
        (bind _output_get (set `self.Count` (- (`self.Count`) 1)))
        (if (<= _output_get 0)
          (`|ExecutionSequence`
            (:`then_0`
              (`self.serverdamage`)))
          (else
            (`/Engine/EditorBlueprintResources/StandardMacros.FlipFlop`
              (:`A`
                (`SceneComponent.SetVisibility` (`self.PointLight`) false false))
              (:`B`
                (`SceneComponent.SetVisibility` (`self.PointLight`) true false)))))))
    (:`then_1`
      (for _array_element (`PrimitiveComponent.GetOverlappingActors` (`self.Box`) null)
        (bind _asbase_character (cast `/Game/Blueprints/Characters/Base_Character` _array_element))
        (if (== (`/Game/Blueprints/Characters/Base_Character.IndexNumber` _asbase_character) 4)
          (if (`/Game/Blueprints/Characters/Base_Character.IsShooting` _asbase_character)
            (`KismetSystemLibrary.Delay` 1.0)
            (bind _asc_player_controller (cast `/Game/Blueprints/Game/C_PlayerController` (`GameplayStatics.GetPlayerController` 0)))
            (`/Engine/EditorBlueprintResources/StandardMacros.IsValid` _asc_player_controller
              (:`Is Valid`
                (bind _returnvalue (`|CreateWidget` "/Game/UI/Ingame/ScreenMessage.ScreenMessage_C" _asc_player_controller "Dynamite Armed.. 30 sec to detonation..."))
                (`UserWidget.AddToViewport` _returnvalue 0)
                (set `self.Blink?` true)
                (`KismetSystemLibrary.Delay` 1.0)
                (`Widget.RemoveFromParent` _returnvalue)
                (set `self.Armed` true)))))))))

(event `ShowAgain`
  (params (player :type "/Game/Blueprints/Characters/Base_Character Object Reference"))
  (`/Engine/EditorBlueprintResources/StandardMacros.IsValid` player
    (:`Is Valid`
      (`KismetSystemLibrary.Delay` 0.5)
      (`SceneComponent.SetVisibility` (`self.DefaultSceneRoot`) true true))))

(fn `UserConstructionScript`
  (`parent.UserConstructionScript`)
  (`SceneComponent.SetVisibility` (`self.PointLight`) false false))
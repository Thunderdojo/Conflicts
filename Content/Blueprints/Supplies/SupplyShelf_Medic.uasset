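; Medic supply shelf that heals characters from a limited stock of health boxes, displayed as four child actors.
; Overlapping its box while below 100 health hides the first available child actor, decrements the stock and adds 20 health.
; Tick re-shows taken boxes while stock suffices, the first three after a delay and the fourth immediately.
; Taken flags are never cleared, as the reset nodes present are unconnected.
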(event `self.Box.OnComponentBeginOverlap`
  (params (OverlappedComponent :type "PrimitiveComponent Object Reference") (OtherActor :type "Actor Object Reference") (OtherComp :type "PrimitiveComponent Object Reference") (OtherBodyIndex :type Integer) (bFromSweep :type Boolean) (SweepResult :type "HitResult Structure (by ref)"))
  (bind _childactor (`self.ChildActor`))
  (bind _childactor1 (`self.ChildActor1`))
  (bind _childactor2 (`self.ChildActor2`))
  ;[1 1 1] Remove boxes after taking
  (bind _asbase_character (cast `/Game/Blueprints/Characters/Base_Character` OtherActor))
  (`/Engine/EditorBlueprintResources/StandardMacros.IsValid` _asbase_character
    (:`Is Valid`
      (if (< (`/Game/Blueprints/Characters/Base_Character.Health` _asbase_character) 100.0)
        (if (`SceneComponent.IsVisible` _childactor)
          (`SceneComponent.SetVisibility` (`self.ChildActor`) false false)
          (set `self.CurrentHealthboxes` (- (`self.CurrentHealthboxes`) 1))
          (set `self.Taken1` true)
          (set `/Game/Blueprints/Characters/Base_Character.Health` (+ (`/Game/Blueprints/Characters/Base_Character.Health` _asbase_character) 20.0) _asbase_character)
          (elif (and (not (`SceneComponent.IsVisible` _childactor)) (`SceneComponent.IsVisible` _childactor1))
            (`SceneComponent.SetVisibility` (`self.ChildActor1`) false false)
            (set `self.CurrentHealthboxes` (- (`self.CurrentHealthboxes`) 1))
            (set `self.Taken2` true)
            (set `/Game/Blueprints/Characters/Base_Character.Health` (+ (`/Game/Blueprints/Characters/Base_Character.Health` _asbase_character) 20.0) _asbase_character)
            (elif (and (not (`SceneComponent.IsVisible` _childactor1)) (`SceneComponent.IsVisible` _childactor2))
              (`SceneComponent.SetVisibility` (`self.ChildActor2`) false false)
              (set `self.CurrentHealthboxes` (- (`self.CurrentHealthboxes`) 1))
              (set `self.Taken3` true)
              (set `/Game/Blueprints/Characters/Base_Character.Health` (+ (`/Game/Blueprints/Characters/Base_Character.Health` _asbase_character) 20.0) _asbase_character)
              (elif (and (not (`SceneComponent.IsVisible` _childactor2)) (`SceneComponent.IsVisible` (`self.ChildActor3`)))
                (`SceneComponent.SetVisibility` (`self.ChildActor3`) false false)
                (set `self.CurrentHealthboxes` (- (`self.CurrentHealthboxes`) 1))
                (set `self.Taken4` true)
                (set `/Game/Blueprints/Characters/Base_Character.Health` (+ (`/Game/Blueprints/Characters/Base_Character.Health` _asbase_character) 20.0) _asbase_character)))))))))

(event `self.ReceiveBeginPlay`
  (set `self.CurrentHealthboxes` (`self.MaxHealthBoxes`)))

(event `self.ReceiveTick`
  (params (DeltaSeconds :type "Float (single-precision)"))
  (if (not (== (`self.CurrentHealthboxes`) 0))
    (`|ExecutionSequence`
      (:`then_0`
        (if (`self.Taken1`)
          (if (> (`self.CurrentHealthboxes`) 0)
            (`KismetSystemLibrary.Delay` 2.0)
            (`SceneComponent.SetVisibility` (`self.ChildActor`) true false))))
      (:`then_1`
        (if (`self.Taken2`)
          (if (> (`self.CurrentHealthboxes`) 1)
            (`KismetSystemLibrary.Delay` 2.0)
            (`SceneComponent.SetVisibility` (`self.ChildActor1`) true false))))
      (:`then_2`
        (if (`self.Taken3`)
          (if (> (`self.CurrentHealthboxes`) 2)
            (`KismetSystemLibrary.Delay` 2.0)
            (`SceneComponent.SetVisibility` (`self.ChildActor2`) true false))))
      (:`then_3`
        (if (`self.Taken4`)
          (if (> (`self.CurrentHealthboxes`) 3)
            (`SceneComponent.SetVisibility` (`self.ChildActor3`) true false)))))))

(fn `UserConstructionScript`)
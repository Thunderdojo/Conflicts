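; Clip is an ammo container that tracks how many rounds it holds and whether it is empty.
; RemoveAmmo subtracts one round per call, and flags the clip empty only when called with none left, not when the last round is removed.
; AddAmmo adds the given amount, clamps the count between zero and the clip's maximum, and always clears the empty flag.
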(fn `AddAmmo`
  (params (AmmoGiven :type Integer))
  (set `self.CurrentAmmoHolding` (`KismetMathLibrary.Clamp` (+ (`self.CurrentAmmoHolding`) AmmoGiven) 0 (`self.MaxAmmoToHold`)))
  (set `self.IsEmpty?` false))

(fn `RemoveAmmo`
  (bind _currentammoholding (`self.CurrentAmmoHolding`))
  (if (< _currentammoholding 1)
    (set `self.IsEmpty?` true)
    (else
      (set `self.CurrentAmmoHolding` (- _currentammoholding 1)))))
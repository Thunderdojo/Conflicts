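; Base constructable placeholder Blueprint that shows a build in progress, then replaces itself with a spawned actor.
; It starts with a hide material and an overlap-only mesh, then switches to a halo material when construction begins.
; On completion it applies the barrier material, blocks all channels, spawns the actor at the mesh's transform and destroys itself after a short delay.
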(event `self.ReceiveBeginPlay`
  (`PrimitiveComponent.SetMaterial` (`self.ConstMesh`) 0 "/Game/Blueprints/Constructables/HideMat.HideMat")
  (`PrimitiveComponent.SetCollisionResponseToAllChannels` (`self.ConstMesh`) "ECR_Overlap"))

(event `BeingConstructed`
  (`PrimitiveComponent.SetMaterial` (`self.ConstMesh`) 0 "/Game/Blueprints/Constructables/ConstructHalo.ConstructHalo"))

(event `Construction_done`
  (params (CrateSpawn :type "Transform Structure"))
  (bind _constmesh (`self.ConstMesh`))
  (set `self.Crate Spawn_0` CrateSpawn)
  (`PrimitiveComponent.SetMaterial` (`self.ConstMesh`) 0 "/Game/Models/constructables/tankbarrier/TankBarrier_M.TankBarrier_M")
  (`PrimitiveComponent.SetCollisionResponseToAllChannels` _constmesh "ECR_Block")
  (`|SpawnActorFromClass` (`self.Class`) (`SceneComponent.K2_GetComponentToWorld` _constmesh) "AdjustIfPossibleButAlwaysSpawn" "OverrideRootScale" null null)
  (`KismetSystemLibrary.Delay` 0.2)
  (`self.K2_DestroyActor`))

(fn `UserConstructionScript`)
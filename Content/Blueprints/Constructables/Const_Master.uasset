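; Master constructable build site: the local player builds a destroyable object by holding fire with the Plier inside its PlierCheck area.
; Tick spawns ClassToSpawn once, passes it respawn transform and class data, and shows a halo material while a tick counter runs.
; At the threshold it clears the halo and destroys the site; releasing fire resets progress and removes the spawned actor.
; The construction script colours the flag and crates by team.
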(event `ServerSetPos`
  (set `self.WorldTransform` (`SceneComponent.K2_GetComponentToWorld` (`self.DefaultSceneRoot`)) :!label _label))

(event `self.ReceiveBeginPlay`
  (goto _label))

(event `self.ReceiveTick`
  (params (DeltaSeconds :type "Float (single-precision)"))
  (bind _placetospawn (`self.PlaceToSpawn`))
  (bind _actorref (`self.ActorRef`))
  (bind _class_to_spawn (`self.Class To Spawn`))
  (bind _asbase_character (cast `/Game/Blueprints/Characters/Base_Character` (`GameplayStatics.GetPlayerPawn` 0)))
  (if (`PrimitiveComponent.IsOverlappingActor` (`self.PlierCheck`) _asbase_character)
    (if (== (`GameplayStatics.GetObjectClass` (`/Game/Blueprints/Characters/Base_Character.GunRef` _asbase_character)) "/Game/Blueprints/Supplies/WeaponBP/Plier.Plier_C")
      (if (`/Game/Blueprints/Characters/Base_Character.IsShooting` _asbase_character)
        (`|ExecutionSequence`
          (:`then_0`
            (`/Engine/EditorBlueprintResources/StandardMacros.DoOnce` false
              (:`Completed`
                (`GameplayStatics.PlaySoundAtLocation` "/Game/Blueprints/Constructables/constSound_Cue.constSound_Cue" (`SceneComponent.K2_GetComponentLocation` (`self.Flag`)) (struct) 1.0 0.0 0.0 null null null))))
          (:`then_1`
            (`/Engine/EditorBlueprintResources/StandardMacros.DoOnce` false
              (:`Completed`
                (`self.ServerSetPos`)
                (bind _returnvalue (`|SpawnActorFromClass` _class_to_spawn (`KismetMathLibrary.MakeTransform` (`KismetMathLibrary.TransformLocation` (`KismetMathLibrary.Conv_VectorToTransform` (`self.K2_GetActorLocation`)) _placetospawn) (`self.Rotation`)) "AlwaysSpawn" "OverrideRootScale" null null))
                (bind _output_get (set `self.ActorRef` _returnvalue))
                (bind _asmaster_destroyable (cast `/Game/Blueprints/Destroyables/Master_Destroyable` _output_get))
                (set `/Game/Blueprints/Destroyables/Master_Destroyable.Set Old Transform` (`self.WorldTransform`) _asmaster_destroyable)
                (set `/Game/Blueprints/Destroyables/Master_Destroyable.PlaceToSpawn` _placetospawn _asmaster_destroyable)
                (set `/Game/Blueprints/Destroyables/Master_Destroyable.Class` _class_to_spawn _asmaster_destroyable)
                (set `/Game/Blueprints/Destroyables/Master_Destroyable.Rotation` (struct) _asmaster_destroyable))))
          (:`then_2`
            (bind _asmaster_destroyable_2 (cast `/Game/Blueprints/Destroyables/Master_Destroyable` (`self.ActorRef`)))
            (`PrimitiveComponent.SetMaterial` (`/Game/Blueprints/Destroyables/Master_Destroyable.DestructableMesh` _asmaster_destroyable_2) 0 "/Game/Blueprints/Constructables/ConstructHalo.ConstructHalo")
            (bind _output_get_2 (set `self.time` (+ (`self.time`) 1)))
            (if (>= _output_get_2 90)
              (bind _asmaster_destroyable_3 (cast `/Game/Blueprints/Destroyables/Master_Destroyable` (`self.ActorRef`)))
              (`PrimitiveComponent.SetMaterial` (`/Game/Blueprints/Destroyables/Master_Destroyable.DestructableMesh` _asmaster_destroyable_3) 0 null)
              (`KismetSystemLibrary.Delay` 0.2)
              (`self.K2_DestroyActor`))))
        (else
          (set `self.time` 0)
          (`/Engine/EditorBlueprintResources/StandardMacros.IsValid` _actorref
            (:`Is Valid`
              (`self.K2_DestroyActor` _actorref)
              (set `self.ActorRef` null))))))))

(fn `UserConstructionScript`
  (bind _cratesandtools (`self.CratesAndTools`))
  (switch `/Game/Blueprints/Game/Teams` (`self.Team`)
    (:`NewEnumerator0`
      (`PrimitiveComponent.SetMaterial` (`self.Flag`) 0 "/Game/Models/constructables/Constructablecrates/Construct.Construct")
      (`PrimitiveComponent.SetMaterial` _cratesandtools 0 "/Game/Models/constructables/Constructablecrates/Construct.Construct"))
    (:`NewEnumerator1`
      (`PrimitiveComponent.SetMaterial` _cratesandtools 0 "/Game/Models/constructables/Constructablecrates/Axis_c.Axis_c")
      (`PrimitiveComponent.SetMaterial` (`self.Flag`) 0 "/Game/Models/constructables/Constructablecrates/Axis_c.Axis_c"))
    (:`NewEnumerator2`
      (`PrimitiveComponent.SetMaterial` _cratesandtools 0 "/Game/Models/constructables/Constructablecrates/Allied_c.Allied_c")
      (`PrimitiveComponent.SetMaterial` (`self.Flag`) 0 "/Game/Models/constructables/Constructablecrates/Allied_c.Allied_c"))))
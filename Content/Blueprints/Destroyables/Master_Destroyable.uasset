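; Master destroyable actor that explodes when its health runs out and leaves a Const_Master actor in its place.
; Box overlap by a player-controlled Base_Character shows a dynamite thumb message, removed after two seconds or on overlap end.
; Damage drains Health; at zero it plays explosion effects, spawns Const_Master using the transform stored by SetTransform, passes on class, placement and rotation data, then destroys itself after a short delay.
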(event `self.Box.OnComponentBeginOverlap`
  (params (OverlappedComponent :type "PrimitiveComponent Object Reference") (OtherActor :type "Actor Object Reference") (OtherComp :type "PrimitiveComponent Object Reference") (OtherBodyIndex :type Integer) (bFromSweep :type Boolean) (SweepResult :type "HitResult Structure (by ref)"))
  (bind _ref (`self.Ref`))
  (bind _asbase_character (cast `/Game/Blueprints/Characters/Base_Character` OtherActor))
  (bind _asc_player_controller (cast `/Game/Blueprints/Game/C_PlayerController` (`Pawn.GetController` _asbase_character)))
  (`/Engine/EditorBlueprintResources/StandardMacros.IsValid` _asc_player_controller
    (:`Is Valid`
      (`/Engine/EditorBlueprintResources/StandardMacros.IsValid` (`self.Ref`)
        (:`Is Not Valid`
          (bind _returnvalue (`|CreateWidget` "/Game/UI/Ingame/ScreenMessageThumb.ScreenMessageThumb_C" _asc_player_controller "" "/Game/UI/Images/Thumbs/Dyno_Thumb2.Dyno_Thumb2"))
          (bind _output_get (set `self.Ref` _returnvalue))
          (`UserWidget.AddToViewport` _output_get 0)
          (`KismetSystemLibrary.Delay` 2.0)
          (`/Engine/EditorBlueprintResources/StandardMacros.IsValid` _ref
            (:`Is Valid`
              (`Widget.RemoveFromParent` _ref)
              (set `self.Ref` null))))))))

(event `self.Box.OnComponentEndOverlap`
  (params (OverlappedComponent :type "PrimitiveComponent Object Reference") (OtherActor :type "Actor Object Reference") (OtherComp :type "PrimitiveComponent Object Reference") (OtherBodyIndex :type Integer))
  (bind _ref (`self.Ref`))
  (`/Engine/EditorBlueprintResources/StandardMacros.IsValid` _ref
    (:`Is Valid`
      (`Widget.RemoveFromParent` _ref)
      (set `self.Ref` null))))

(event `SetTransform`
  (params (SetOldTransform :type "Transform Structure"))
  (set `self.Set Old Transform` SetOldTransform))

(event `self.ReceiveAnyDamage`
  (params (Damage :type "Float (single-precision)") (DamageType :type "DamageType Object Reference") (InstigatedBy :type "Controller Object Reference") (DamageCauser :type "Actor Object Reference"))
  (bind _returnvalue (`SceneComponent.K2_GetComponentLocation` (`self.DefaultSceneRoot`)))
  (bind _output_get (set `self.Health` (- (`self.Health`) Damage)))
  (if (<= _output_get 0.0)
    (`GameplayStatics.PlaySoundAtLocation` "/Game/Audio/Explosion01.Explosion01" _returnvalue (struct) 1.0 1.0 0.0 null null null)
    (`GameplayStatics.SpawnEmitterAtLocation` "/Game/Particles/P_Explosion.P_Explosion" _returnvalue (struct) (4.0 4.0 4.0))
    (bind _returnvalue_2 (`|SpawnActorFromClass` "/Game/Blueprints/Constructables/Const_Master.Const_Master_C" (`self.Set Old Transform`) "Undefined" "OverrideRootScale" null (`SceneComponent.K2_GetComponentToWorld` (`self.DefaultSceneRoot`)) (`self.Class`) null))
    (set `/Game/Blueprints/Constructables/Const_Master.PlaceToSpawn` (`self.PlaceToSpawn`) _returnvalue_2)
    (set `/Game/Blueprints/Constructables/Const_Master.Rotation` (`self.Rotation`) _returnvalue_2)
    (`KismetSystemLibrary.Delay` 0.2)
    (`self.K2_DestroyActor`)))

(fn `UserConstructionScript`)